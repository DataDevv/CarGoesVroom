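; BP_Porche911GT3 is a drivable Porsche 911 GT3 vehicle that applies player input to driving and camera rotation every Tick.
; VehicleMovement feeds the throttle and brake axes into the vehicle movement component.
; Steering and handbrake calls are unconnected and never run; steering there reads MoveForward, while MoveRight is unused.
; VehicleCamera rotates the spring arm from the LookUp and LookRight axes.
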(event `self.ReceiveTick`
  (params (DeltaSeconds :type "Float (single-precision)"))
  (`self.Vehicle_Movement`)
  (`self.Vehicle_Camera`))

(fn `UserConstructionScript`)

(fn `Vehicle_Camera`
  (`SceneComponent.K2_AddRelativeRotation` (`self.SpringArm`) (`KismetMathLibrary.MakeRotator` 0.0 (`self.GetInputAxisValue`) (`self.GetInputAxisValue`)) false false))

(fn `Vehicle_Movement`
  (bind _vehiclemovementcomponent (`self.VehicleMovementComponent`))
  (`ChaosVehicleMovementComponent.SetThrottleInput` _vehiclemovementcomponent (`self.GetInputAxisValue`))
  (`ChaosVehicleMovementComponent.SetBrakeInput` _vehiclemovementcomponent (`self.GetInputAxisValue`)))