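; Temporary Porsche 911 GT3 vehicle Blueprint that drives from input and experiments with detecting nearby actors.
; Each Tick feeds throttle, brake and steering axes to the movement component, keeps the handbrake off, and rotates the spring arm from look input.
; It also runs a debug-drawn sphere trace and a sphere overlap, both with velocity-scaled radius.
; For each overlapped actor, a look-at rotation check decides whether "Turn Left" prints on screen.
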(event `self.ReceiveTick`
  (params (DeltaSeconds :type "Float (single-precision)"))
  (bind _mesh (`self.Mesh`))
  (bind _returnvalue (`SceneComponent.K2_GetComponentLocation` _mesh))
  (bind _returnvalue_2 (`KismetMathLibrary.VSize` (* (`SceneComponent.GetComponentVelocity` _mesh) (`self.Radius`))))
  (`self.Vehicle_Movement`)
  (`self.Vehicle_Camera`)
  (`KismetSystemLibrary.SphereTraceMulti` :`Start` _returnvalue :`End` _returnvalue :`Radius` _returnvalue_2 :`TraceChannel` "TraceTypeQuery1" :`DrawDebugType` "ForOneFrame")
  (bind _outactors (`KismetSystemLibrary.SphereOverlapActors` _returnvalue _returnvalue_2 (`self.objectType`)))
  (for _array_element _outactors
    (`KismetSystemLibrary.PrintString` "Turn Left" (> (.y (`KismetMathLibrary.Conv_RotatorToVector` (`KismetMathLibrary.FindLookAtRotation` (`KismetMathLibrary.RotateAngleAxis` _returnvalue (`KismetMathLibrary.RadiansToDegrees` (.y (`KismetMathLibrary.Conv_RotatorToVector` (`SceneComponent.K2_GetComponentRotation` (`self.Mesh`)))))) (`self.K2_GetActorLocation` _array_element)))) 0.0))))

(fn `UserConstructionScript`)

(fn `Vehicle_Camera`
  (`SceneComponent.K2_AddRelativeRotation` (`self.SpringArm`) (`KismetMathLibrary.MakeRotator` 0.0 (`self.GetInputAxisValue`) (`self.GetInputAxisValue`)) false false))

(fn `Vehicle_Movement`
  (bind _vehiclemovementcomponent (`self.VehicleMovementComponent`))
  (`ChaosVehicleMovementComponent.SetThrottleInput` _vehiclemovementcomponent (`self.GetInputAxisValue`))
  (`ChaosVehicleMovementComponent.SetBrakeInput` _vehiclemovementcomponent (`self.GetInputAxisValue`))
  (`ChaosVehicleMovementComponent.SetSteeringInput` _vehiclemovementcomponent (`self.GetInputAxisValue`))
  (`ChaosVehicleMovementComponent.SetHandbrakeInput` _vehiclemovementcomponent false))