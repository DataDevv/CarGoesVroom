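; Home building that serves as a delivery destination for the player's Porsche 911 GT3 or Starship.
; Every tick, a debug-drawn box trace offset along the mesh's right vector looks for either vehicle, checking for Starship only without a valid Porsche actor.
; If the detected vehicle's order matches this Address and has time left, it earns the price plus remaining seconds, then its order and arrow flag are cleared.
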(event `self.ReceiveTick`
  (params (DeltaSeconds :type "Float (single-precision)"))
  (bind _playerstarship (`self.PlayerStarship`))
  (bind _playerstarship_2 (`self.PlayerStarship`))
  (bind _playerporshe (`self.PlayerPorshe`))
  (bind _playerporshe_2 (`self.PlayerPorshe`))
  (bind (_address _price _timeleft) (break `/Game/Blueprints/Struct_Order` (`/Game/Vehicles/Imported_Vehicle/BP_Porche911GT3.Orders` _playerporshe)))
  (bind (_address_2 _price_2 _timeleft_2) (break `/Game/Blueprints/Struct_Order` (`/Game/Vehicles/starship-delivery-robot-model/BP_Starship.Orders` _playerstarship)))
  (bind _returnvalue (`KismetMathLibrary.GetTotalSeconds` _timeleft_2))
  (bind _returnvalue_2 (`KismetMathLibrary.GetTotalSeconds` _timeleft))
  (bind _returnvalue_3 (+ (+ (`SceneComponent.K2_GetComponentLocation` (`self.StaticMesh`)) (* (`SceneComponent.GetRightVector` (`self.StaticMesh`)) (4000.0 4000.0 1.0))) (0.0 0.0 100.0)))
  ;[1 1 1] Creating detection box to detect the players car
  (set `self.PlayerPorshe` null)
  (bind _outhits (`KismetSystemLibrary.BoxTraceMulti` :`Start` _returnvalue_3 :`End` _returnvalue_3 :`HalfSize` (400.0 400.0 100.0) :`Orientation` (`SceneComponent.K2_GetComponentRotation` (`self.StaticMesh`)) :`TraceChannel` "TraceTypeQuery1" :`DrawDebugType` "ForOneFrame"))
  ;[1 1 1] Detecting whether the player is using a Starship or a Porsche
  (for _array_element _outhits
    (bind _returnvalue_4 (`GameplayStatics.GetActorOfClass` "/Game/Vehicles/Imported_Vehicle/BP_Porche911GT3.BP_Porche911GT3_C"))
    (if (`KismetSystemLibrary.IsValid` _returnvalue_4)
      (bind (_bblockinghit _binitialoverlap _time _distance _location _impactpoint _normal _impactnormal _physmat _hitactor) (`GameplayStatics.BreakHitResult` _array_element))
      (if (== _returnvalue_4 _hitactor)
        (set `self.PlayerPorshe` _returnvalue_4))
      (else
        (bind _returnvalue_5 (`GameplayStatics.GetActorOfClass` "/Game/Vehicles/starship-delivery-robot-model/BP_Starship.BP_Starship_C"))
        (if (== _returnvalue_5 _hitactor)
          (set `self.PlayerStarship` _returnvalue_5)))))
  ;[1 0.3722 0.3024] Checking to see if the player has an active order, and if so, if that order is correct to the house
  (if (`KismetSystemLibrary.IsValid` (`self.PlayerPorshe`))
    (if (== _address (`self.Address`))
      (if (> _returnvalue_2 0.0)
        (set `/Game/Vehicles/Imported_Vehicle/BP_Porche911GT3.Money` (+ _price (`/Game/Vehicles/Imported_Vehicle/BP_Porche911GT3.Money` _playerporshe) _returnvalue_2) _playerporshe_2)
        (set `/Game/Vehicles/Imported_Vehicle/BP_Porche911GT3.Orders` (struct) _playerporshe_2)
        (set `/Game/Vehicles/Imported_Vehicle/BP_Porche911GT3.NeedsArrow` false _playerporshe_2)))
    (else
      ;[1 1 1] Same as above but using the starship instead of the porsche
      (if (`KismetSystemLibrary.IsValid` _playerstarship)
        (if (== _address_2 (`self.Address`))
          (if (> _returnvalue 0.0)
            (set `/Game/Vehicles/starship-delivery-robot-model/BP_Starship.Money` (+ _price_2 (`/Game/Vehicles/starship-delivery-robot-model/BP_Starship.Money` _playerstarship) _returnvalue) _playerstarship_2)
            (set `/Game/Vehicles/starship-delivery-robot-model/BP_Starship.Orders` (struct) _playerstarship_2)
            (set `/Game/Vehicles/starship-delivery-robot-model/BP_Starship.NeedsArrow` false _playerstarship_2)))))))

(fn `UserConstructionScript`)