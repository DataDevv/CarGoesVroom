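; Cafe building actor that gives the player's Porsche a delivery-style order when the car is in its pickup zone.
; Each Tick runs a debug-drawn box trace at an offset from the mesh and matches hits against the first BP_Porche911GT3 found in the world.
; A detected car receives a hardcoded test order, unless its Orders array already holds that order ID.
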(event `self.ReceiveTick`
  (params (DeltaSeconds :type "Float (single-precision)"))
  (bind _orders (`/Game/Vehicles/Imported_Vehicle/BP_Porche911GT3.Orders` (`self.PlayerPorshe`)))
  (bind _returnvalue (+ (+ (`SceneComponent.K2_GetComponentLocation` (`self.StaticMesh`)) (* (`SceneComponent.GetForwardVector` (`self.StaticMesh`)) (-1300.0 -1300.0 1.0))) (0.0 0.0 100.0)))
  (set `self.HasOrder` false)
  (set `self.PlayerPorshe` null)
  (bind _outhits (`KismetSystemLibrary.BoxTraceMulti` :`Start` _returnvalue :`End` _returnvalue :`HalfSize` (400.0 400.0 100.0) :`Orientation` (`SceneComponent.K2_GetComponentRotation` (`self.StaticMesh`)) :`TraceChannel` "TraceTypeQuery1" :`DrawDebugType` "ForOneFrame"))
  (for _array_element _outhits
    (bind _returnvalue_2 (`GameplayStatics.GetActorOfClass` "/Game/Vehicles/Imported_Vehicle/BP_Porche911GT3.BP_Porche911GT3_C"))
    (if (== _returnvalue_2 (`.HitActor` (`GameplayStatics.BreakHitResult` _array_element)))
      (set `self.PlayerPorshe` _returnvalue_2)))
  (if (`KismetSystemLibrary.IsValid` (`self.PlayerPorshe`))
    (for _array_element_2 _orders
      (if (== (`.OrderID_13_B6D3600C424BD7B0F44849AE563892CA` (break `/Game/Blueprints/Struct_Order` _array_element_2)) 1)
        (set `self.HasOrder` true)))
    (if (not (`self.HasOrder`))
      (`KismetArrayLibrary.Array_Add` _orders (make `/Game/Blueprints/Struct_Order` "Test Address" 100.0 (struct) 1))
      (set `/Game/Vehicles/Imported_Vehicle/BP_Porche911GT3.Orders` _orders (`self.PlayerPorshe`)))))

(fn `UserConstructionScript`)