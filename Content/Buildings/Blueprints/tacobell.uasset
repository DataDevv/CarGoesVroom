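; Taco Bell building actor that opens an ordering menu when the player drives or flies up in the Porsche or starship.
; Each Tick, a debug-drawn box trace around the static mesh compares hits against the level's Porsche, or the starship if no Porsche exists.
; A match creates the TacoBellOrders widget and shows the mouse cursor; losing it removes both.
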(event `self.ReceiveTick`
  (params (DeltaSeconds :type "Float (single-precision)"))
  (bind _returnvalue (`GameplayStatics.GetPlayerController` 0))
  (bind _orderwidget (`self.OrderWidget`))
  (bind _returnvalue_2 (`SceneComponent.K2_GetComponentLocation` (`self.StaticMesh`)))
  ;[1 1 1] Creating detection box to detect player
  (set `self.HasOrder` false)
  (set `self.PlayerStarship` null)
  (set `self.PlayerPorshe` null)
  (bind _outhits (`KismetSystemLibrary.BoxTraceMulti` :`Start` _returnvalue_2 :`End` _returnvalue_2 :`HalfSize` (3500.0 3500.0 2000.0) :`Orientation` (`SceneComponent.K2_GetComponentRotation` (`self.StaticMesh`)) :`TraceChannel` "TraceTypeQuery1" :`DrawDebugType` "ForOneFrame"))
  ;[1 1 1] Determines if the player is in a starship or porsche
  (for _array_element _outhits
    (bind _returnvalue_3 (`GameplayStatics.GetActorOfClass` "/Game/Vehicles/Imported_Vehicle/BP_Porche911GT3.BP_Porche911GT3_C"))
    (if (`KismetSystemLibrary.IsValid` _returnvalue_3)
      (bind (_bblockinghit _binitialoverlap _time _distance _location _impactpoint _normal _impactnormal _physmat _hitactor) (`GameplayStatics.BreakHitResult` _array_element))
      (if (== _returnvalue_3 _hitactor)
        (set `self.PlayerPorshe` _returnvalue_3))
      (else
        (bind _returnvalue_4 (`GameplayStatics.GetActorOfClass` "/Game/Vehicles/starship-delivery-robot-model/BP_Starship.BP_Starship_C"))
        (if (== _returnvalue_4 _hitactor)
          (set `self.PlayerStarship` _returnvalue_4)))))
  (if (`KismetSystemLibrary.IsValid` (`self.PlayerPorshe`))
    ;[1 1 1] If the user does not have the menu opened, open it
    (if (not (`KismetSystemLibrary.IsValid` (`self.OrderWidget`))) :!label _label
      (bind _returnvalue_5 (`|CreateWidget` "/Game/UI/TacoBellOrders.TacoBellOrders_C" (`GameplayStatics.GetPlayerController` 0)))
      (`/Game/UI/TacoBellOrders.Opened` _returnvalue_5)
      (`UserWidget.AddToViewport` _returnvalue_5 0)
      (set `self.OrderWidget` _returnvalue_5)
      (set `PlayerController.bShowMouseCursor` true _returnvalue))
    (elif (`KismetSystemLibrary.IsValid` (`self.PlayerStarship`))
      (goto _label)
      (else
        ;[1 1 1] Close whenever the player leaves
        (if (`KismetSystemLibrary.IsValid` _orderwidget)
          (`Widget.RemoveFromParent` _orderwidget)
          (set `self.OrderWidget` null)
          (set `PlayerController.bShowMouseCursor` false _returnvalue))))))

(fn `UserConstructionScript`)